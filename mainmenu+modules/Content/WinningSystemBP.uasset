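; WinningSystemBP tracks minigame progress and decides whether to open the win panel, the lose panel or return to FirstPersonMap.
; AddCompletedGame increments both completed and total counts, then runs CheckWinCondition.
; That check requires each of five minigame counters (Decoding, Sequence, Puzzle, MemoryCards, ConnectWires) before comparing totals against win and loss thresholds.
; Missing types reload the map, but too few total games triggers no level change.
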(event EventBeginPlay)

(event Collision|EventActorBeginOverlap
  (params (OtherActor :type Actor%20Object%20Reference)))

(event EventTick
  (params (DeltaSeconds :type Float%20%28single-precision%29)))

(fn ConstructionScript)

(fn AddCompletedGame
  (bind _result (Math|Integer|IncrementInt (Variables|Default|GetCompleted_Games))
    (:%20%20
      (Variables|Default|SetCompleted_Games _result)
      (bind _result_2 (Math|Integer|IncrementInt (Variables|Default|GetTotalGamesPlayed))
        (:%20%20
          (Variables|Default|SetTotalGamesPlayed _result_2)
          (CallFunction|CheckWinCondition))))))

(fn CheckWinCondition
  (if (>= (Variables|Default|Getdecoding) 1)
    (if (>= (Variables|Default|Getsequence) 1)
      (if (>= (Variables|Default|Getpuzzle) 1)
        (if (>= (Variables|Default|Getmemory_cards) 1)
          (if (>= (Variables|Default|Getconnect_wires) 1)
            (if (>= (Variables|Default|GetTotalGamesPlayed) 5)
              (if (>= (Variables|Default|GetCompleted_Games) 3)
                (Game|OpenLevel(byName) "Win_Panel")
                (elif (>= (Variables|Default|GetTotalGamesPlayed) 10)
                  (Game|OpenLevel(byName) "Loose_Panel")
                  (else
                    (Development|PrintString "Hello")
                    (Game|OpenLevel(byName) "FirstPersonMap")))))
            (else
              (Development|PrintString (Utilities|String|ToString(Integer) (Variables|Default|GetCompleted_Games)) :!label _label)
              (Game|OpenLevel(byName) "FirstPersonMap")))
          (else
            (goto _label)))
        (else
          (goto _label)))
      (else
        (goto _label)))
    (else
      (goto _label))))