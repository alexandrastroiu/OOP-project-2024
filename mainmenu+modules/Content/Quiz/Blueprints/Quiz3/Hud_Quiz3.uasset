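; Quiz 3 controller that shows the QuestionWidget3 UI on BeginPlay, with UI-only input and a visible cursor.
; EventNextQuestion calls NextQuestion, then feeds the widget the next entry from the Question array.
; Score increments on every call, including the initial one, because its branch is fixed to true rather than reading AnswerCorrect.
; When questions run out, it opens the SequenceRepeat level and restores game-and-UI input.
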(event Custom|EventNextQuestion
  (params (AnswerCorrect :type Boolean))
  (bind _currentquestion (Variables|Default|GetCurrentQuestion))
  (CallFunction|NextQuestion AnswerCorrect)
  (if true
    (Math|Integer|IncrementInt (Variables|Default|GetScore)
      (:%20%20
        _)))
  (if (>= (Utilities|Array|LastIndex (Variables|Default|GetQuestion)) _currentquestion)
    (Default|InitQuestion (Variables|Default|GetQuestionWidget) (Utilities|Array|Get(acopy) (Variables|Default|GetQuestion) _currentquestion))
    (Math|Integer|IncrementInt _currentquestion)
    (else
      (Game|OpenLevel(byName) "SequenceRepeat")
      (Input|SetInputModeGameandUI (Game|GetPlayerController 0) 0 "DoNotLock" true false))))

(event EventBeginPlay
  (bind _returnvalue (Game|GetPlayerController 0))
  (bind _returnvalue_2 (UserInterface|CreateWidget "/Game/Quiz/Blueprints/Quiz3/QuestionWidget3.QuestionWidget3_C"))
  (bind _output_get (Variables|Default|SetQuestionWidget _returnvalue_2))
  (UserInterface|Viewport|AddtoViewport _output_get 0)
  (Input|SetInputModeUIOnly _returnvalue _output_get "DoNotLock" false)
  (Variables|/Script/Engine.PlayerController|SetbShowMouseCursor _returnvalue true)
  (CallFunction|EventNextQuestion false))

(event Collision|EventActorBeginOverlap
  (params (OtherActor :type Actor%20Object%20Reference)))

(event EventTick
  (params (DeltaSeconds :type Float%20%28single-precision%29)))

(fn ConstructionScript)