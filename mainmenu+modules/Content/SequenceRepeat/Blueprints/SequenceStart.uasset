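; Controller actor for a Simon-style sequence-repeat minigame, started by clicking it and played across linked note buttons.
; Per-level settings drive a random note sequence, built and played back through delayed self-calling events.
; Player notes are checked in order: mistakes restart the level with a new sequence, successes advance it, and the final win opens FirstPersonMap.
; The construction script caps note counts to the button count when duplicates are disallowed.
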(event OnClicked(SequenceStart)
  (params (TouchedComponent :type Primitive%20Component%20Object%20Reference) (ButtonPressed :type Key%20Structure :default "None"))
  (if (not (Variables|Default|GetisPlaying))
    (Variables|Default|SetisPlaying true)
    (CallFunction|StartLevel)))

(event Custom|StartLevel
  (Utilities|Array|Clear (Variables|Default|GetPlayerSequence))
  (Variables|Default|SetCurrentNote 0)
  (Variables|Default|SetisPlayersTurn false)
  (CallFunction|CreateSequence))

(event Custom|CreateSequence
  (bind _levelsettings (Variables|Default|GetLevelSettings))
  (bind _currentlevel (Variables|Default|GetCurrentLevel))
  (bind _output (Utilities|Array|Get(acopy) _levelsettings _currentlevel))
  (bind (_numberofnotes _timebetween _canduplicatenotes) (Utilities|Struct|BreakSequenceLevel_Struct _output))
  (Utilities|Array|Clear (Variables|Default|GetGameSequence))
  (if (> (Utilities|Array|Length (Variables|Default|GetButton)) 0)
    (if _canduplicatenotes
      (Utilities|Array|Add (Variables|Default|GetGameSequence) (Math|Random|RandomIntegerinRange 0 (Utilities|Array|LastIndex (Variables|Default|GetButton))))
      (else
        (Utilities|Array|AddUnique (Variables|Default|GetGameSequence) (Math|Random|RandomIntegerinRange 0 (Utilities|Array|LastIndex (Variables|Default|GetButton))))))
    (if (< (Utilities|Array|Length (Variables|Default|GetGameSequence)) _numberofnotes)
      (Utilities|FlowControl|Delay 0.0)
      (CallFunction|AddAnotherNote)
      (else
        (Utilities|FlowControl|Delay 1.0)
        (CallFunction|PlayGameSequence)))))

(event Custom|AddAnotherNote
  (bind _levelsettings (Variables|Default|GetLevelSettings))
  (bind _currentlevel (Variables|Default|GetCurrentLevel))
  (bind _output (Utilities|Array|Get(acopy) _levelsettings _currentlevel))
  (bind (_numberofnotes _timebetween _canduplicatenotes) (Utilities|Struct|BreakSequenceLevel_Struct _output))
  (if (> (Utilities|Array|Length (Variables|Default|GetButton)) 0)
    (if _canduplicatenotes
      (Utilities|Array|Add (Variables|Default|GetGameSequence) (Math|Random|RandomIntegerinRange 0 (Utilities|Array|LastIndex (Variables|Default|GetButton))))
      (else
        (Utilities|Array|AddUnique (Variables|Default|GetGameSequence) (Math|Random|RandomIntegerinRange 0 (Utilities|Array|LastIndex (Variables|Default|GetButton))))))
    (if (< (Utilities|Array|Length (Variables|Default|GetGameSequence)) _numberofnotes)
      (Utilities|FlowControl|Delay 0.0)
      (CallFunction|AddAnotherNote)
      (else
        (Utilities|FlowControl|Delay 1.0)
        (CallFunction|PlayGameSequence)))))

(event Custom|Play%20Game%20Sequence
  (Default|PlayNote (Utilities|Array|Get(acopy) (Variables|Default|GetButton) (Utilities|Array|Get(acopy) (Variables|Default|GetGameSequence) (Variables|Default|GetCurrentNote))))
  (Utilities|FlowControl|Delay (Utilities|Struct|BreakSequenceLevel_Struct (Utilities|Array|Get(acopy) (Variables|Default|GetLevelSettings) (Variables|Default|GetCurrentLevel))))
  (Math|Integer|IncrementInt (Variables|Default|GetCurrentNote)
    (:%20%20
      (if (< (Variables|Default|GetCurrentNote) (Utilities|Array|Length (Variables|Default|GetGameSequence)))
        (CallFunction|PlayGameSequence)
        (else
          (Variables|Default|SetisPlayersTurn true))))))

(event Custom|PlayerPlayedNote
  (params (Note :type Integer))
  (Variables|Default|SetisPlayersTurn false)
  (bind _returnvalue (Utilities|Array|Add (Variables|Default|GetPlayerSequence) Note))
  (if (== Note (Utilities|Array|Get(acopy) (Variables|Default|GetGameSequence) _returnvalue))
    (Default|PlayNote (Utilities|Array|Get(acopy) (Variables|Default|GetButton) (Utilities|Array|Get(acopy) (Variables|Default|GetGameSequence) _returnvalue)))
    (if (>= (Utilities|Array|Length (Variables|Default|GetPlayerSequence)) (Utilities|Array|Length (Variables|Default|GetGameSequence)))
      (if (< (Variables|Default|GetCurrentLevel) (Utilities|Array|LastIndex (Variables|Default|GetLevelSettings)))
        (Math|Integer|IncrementInt (Variables|Default|GetCurrentLevel)
          (:%20%20
            (Utilities|FlowControl|Delay 2.0)
            (CallFunction|StartLevel)))
        (else
          (Development|PrintString "You Win!")
          (Game|OpenLevel(byName) "FirstPersonMap")
          (Input|SetInputModeGameandUI (Game|GetPlayerController 0) 0 "DoNotLock" true false)))
      (else
        (Variables|Default|SetisPlayersTurn true)))
    (else
      (for _array_element (Variables|Default|GetButton)
        _)
      (Utilities|FlowControl|Delay 0.2)
      (CallFunction|StartLevel))))

(event EventBeginPlay
  (Variables|/Script/Engine.PlayerController|SetbShowMouseCursor (Game|GetPlayerController 0) true)
  (for _array_element (Variables|Default|GetButton)
    (Utilities|IsValid _array_element
      (:Is%20Valid
        (Variables|/Game/SequenceRepeat/Blueprints/SequenceButton.SequenceButton_C|SetSequenceMain_Ref _array_element self))
      (:Is%20Not%20Valid
        (Development|PrintString "set up buttons")))))

(event Collision|EventActorBeginOverlap
  (params (OtherActor :type Actor%20Object%20Reference)))

(event EventTick
  (params (DeltaSeconds :type Float%20%28single-precision%29)))

(fn ConstructionScript
  (bind _button (Variables|Default|GetButton))
  (bind _returnvalue (Utilities|Array|Length _button))
  (for (_array_element _array_index) (Variables|Default|GetLevelSettings)
    (if (not (.CanDuplicateNotes (Utilities|Struct|BreakSequenceLevel_Struct _array_element)))
      (if (> (.NumberOfNotes (Utilities|Struct|BreakSequenceLevel_Struct _array_element)) _returnvalue)
        (bind _structout (Utilities|Struct|SetmembersinSequenceLevel_Struct _array_element _returnvalue))
        (Utilities|Array|SetArrayElem (Variables|Default|GetLevelSettings) _array_index _structout)))))