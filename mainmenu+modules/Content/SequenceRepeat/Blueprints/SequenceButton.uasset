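; SequenceButton is an interactable colored button that plays its own sound and flashes, apparently for a sequence-repeat minigame.
; The construction script creates a dynamic instance of M_Color tinted with its Color variable, and BeginPlay assigns its Sound to the audio component.
; OnInteract, from an actor implementing BPI_Player, calls PlayNote, which starts the audio and raises material Intensity, then resets both after a brief delay.
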(event Custom|PlayNote
  (Audio|Components|Audio|Play (Variables|Default|GetAudio) 0.0)
  (Rendering|Material|SetScalarParameterValue (Variables|Default|GetDyn%20Mat) "Intensity" 2.5 :!class /Script/Engine.MaterialInstanceDynamic)
  (Utilities|FlowControl|Delay 0.2)
  (Audio|Components|Audio|Stop (Variables|Default|GetAudio))
  (Rendering|Material|SetScalarParameterValue (Variables|Default|GetDyn%20Mat) "Intensity" 0.0 :!class /Script/Engine.MaterialInstanceDynamic))

(event Collision|EventActorBeginOverlap
  (params (OtherActor :type Actor%20Object%20Reference)))

(event EventTick
  (params (DeltaSeconds :type Float%20%28single-precision%29)))

(event EventOnInteract
  (params (Actor :type Actor%20Object%20Reference))
  (if (Utilities|DoesObjectImplementInterface Actor "/Game/SequenceRepeat/Blueprints/Interfaces/BPI_Player.BPI_Player_C")
    (if true
      (CallFunction|PlayNote))))

(event EventBeginPlay
  (Audio|Components|Audio|SetSound (Variables|Default|GetAudio) (Variables|Default|GetSound)))

(event EventOnLookat
  (params (Actor :type Actor%20Object%20Reference)))

(fn ConstructionScript
  (bind _returnvalue (Rendering|Material|CreateDynamicMaterialInstance (Variables|Default|GetSequenceButton) 0 "/Game/SequenceRepeat/Materials/M_Color.M_Color" "None" :!class /Script/Engine.PrimitiveComponent))
  (bind _output_get (Variables|Default|SetDyn%20Mat _returnvalue))
  (Rendering|Material|SetVectorParameterValue _output_get "Color" (Variables|Default|GetColor) :!class /Script/Engine.MaterialInstanceDynamic))

(fn NewFunction)